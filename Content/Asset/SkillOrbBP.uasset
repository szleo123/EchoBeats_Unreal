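; Skill orb Blueprint that shows the three most recent skill key presses as orbiting orbs.
; Tick advances a phase that places the orbs a third of a turn apart on a flat circle, using sine and cosine with swept relative moves.
; UpdateOrbSkill resets materials to FrameMaterial, then colors orbs newest-first through EBGameMode's KeyMatMapping, leaving unused orbs on the frame material.
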(event `self.ReceiveBeginPlay`
  (`self.ClearMat`)
  (`self.UpdateOrbLoc`))

(event `self.ReceiveTick`
  (params (DeltaSeconds :type "Float (single-precision)"))
  (set `self.Prog` (+ (* DeltaSeconds 2.5) (`self.Prog`)))
  (`self.UpdateOrbLoc`))

(fn `ClearMat`
  (`KismetArrayLibrary.Array_Set` (`self.Mats`) 0 "/Engine/VREditor/UI/FrameMaterial.FrameMaterial")
  (`KismetArrayLibrary.Array_Set` (`self.Mats`) 1 "/Engine/VREditor/UI/FrameMaterial.FrameMaterial")
  (`KismetArrayLibrary.Array_Set` (`self.Mats`) 2 "/Engine/VREditor/UI/FrameMaterial.FrameMaterial"))

(fn `GetLocOnProg`
  (params (Prog :type "Float (double-precision)") (Radius :type "Float (double-precision)"))
  (returns (Location :type "Vector Structure"))
  (return (`KismetMathLibrary.MakeVector` (* Radius (`KismetMathLibrary.Sin` Prog)) (* (`KismetMathLibrary.Cos` Prog) Radius))))

(fn `GetSkillMat`
  (params (Skill :type "Array of /Game/DataStruct/SkillKeyPress Structure") (`Reverse Index` :type Integer))
  (returns (Value :type "MaterialInstance Object Reference"))
  (bind _output_key (break `/Game/DataStruct/SkillKeyPress` (`|GetArrayItem` Skill (- (`KismetArrayLibrary.Array_Length` Skill) `Reverse Index` 1))))
  (return (`BlueprintMapLibrary.Map_Find` (`/Game/Characters/EBGameMode.KeyMatMapping` (cast `/Game/Characters/EBGameMode` (`GameplayStatics.GetGameMode`) :!pure true)) _output_key)))

(fn `SetOrbMaterial`
  (`PrimitiveComponent.SetMaterial` (`self.Orb1`) 0 (`|GetArrayItem` (`self.Mats`)))
  (`PrimitiveComponent.SetMaterial` (`self.Orb2`) 0 (`|GetArrayItem` (`self.Mats`) 1))
  (`PrimitiveComponent.SetMaterial` (`self.Orb3`) 0 (`|GetArrayItem` (`self.Mats`) 2)))

(fn `UpdateOrbLoc`
  (`SceneComponent.K2_SetRelativeLocation` (`self.Orb2`) (`self.GetLocOnProg` (`self.Prog`) (`self.Radius`)) true false)
  (`SceneComponent.K2_SetRelativeLocation` (`self.Orb1`) (`self.GetLocOnProg` (+ (`self.Prog`) 2.09) (`self.Radius`)) true false)
  (`SceneComponent.K2_SetRelativeLocation` (`self.Orb3`) (`self.GetLocOnProg` (+ (`self.Prog`) 4.18) (`self.Radius`)) true false))

(fn `UpdateOrbSkill`
  (params (Skills :type "Array of /Game/DataStruct/SkillKeyPress Structure"))
  (locals (KeyPressArray :type "Array of /Game/DataStruct/SkillKeyPress Structure"))
  (bind _output_get (set `local.KeyPressArray` Skills))
  (`self.ClearMat`)
  (switch `int` (`KismetArrayLibrary.Array_Length` _output_get)
    (:`Default`
      (`KismetArrayLibrary.Array_Set` (`self.Mats`) 2 (`self.GetSkillMat` (`local.KeyPressArray`) 2))
      (`KismetArrayLibrary.Array_Set` (`self.Mats`) 1 (`self.GetSkillMat` (`local.KeyPressArray`) 1) :!label _label)
      (`KismetArrayLibrary.Array_Set` (`self.Mats`) 0 (`self.GetSkillMat` (`local.KeyPressArray`)) :!label _label_2)
      (`self.SetOrbMaterial`))
    (:`0`
      (`self.SetOrbMaterial`))
    (:`1`
      (goto _label_2))
    (:`2`
      (goto _label))))

(fn `UserConstructionScript`)