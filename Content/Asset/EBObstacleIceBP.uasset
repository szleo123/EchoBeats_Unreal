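; Obstacle actor with an element, destroyed when hit by a spell that counters that element.
; SetElement applies the element's material from the game mode's SkillMatMapping, on construction and at BeginPlay.
; On Hit by a spelllBP, it looks up the spell in SkillCounterMapping and destroys itself on a match; the spell is destroyed either way.
; The React function is an empty stub.
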(event `self.ReceiveBeginPlay`
  (`self.SetElement`))

(event `self.ReceiveHit`
  (params (MyComp :type "PrimitiveComponent Object Reference") (Other :type "Actor Object Reference") (OtherComp :type "PrimitiveComponent Object Reference") (bSelfMoved :type Boolean) (HitLocation :type "Vector Structure") (HitNormal :type "Vector Structure") (NormalImpulse :type "Vector Structure") (Hit :type "HitResult Structure (by ref)"))
  (bind _asspelll_bp (cast `/Game/Asset/spelllBP` Other))
  (if (`|EnumEquality` (`self.Element`) (`BlueprintMapLibrary.Map_Find` (`/Game/Characters/EBGameMode.SkillCounterMapping` (`self.GetGameMode`)) (`/Game/Asset/spelllBP.Spell` _asspelll_bp)))
    (`self.K2_DestroyActor`)
    (`KismetSystemLibrary.PrintText` "Dest"))
  (`self.K2_DestroyActor` _asspelll_bp))

(fn `GetGameMode`
  (returns (`AsEBGame Mode` :type "/Game/Characters/EBGameMode Object Reference"))
  (return (cast `/Game/Characters/EBGameMode` (`GameplayStatics.GetGameMode`) :!pure true)))

(fn `React`
  (params (NewParam :type Boolean)))

(fn `SetElement`
  (`PrimitiveComponent.SetMaterial` (`self.StaticMesh`) 0 (`BlueprintMapLibrary.Map_Find` (`/Game/Characters/EBGameMode.SkillMatMapping` (`self.GetGameMode`)) (`self.Element`))))

(fn `UserConstructionScript`
  (`self.SetElement`))