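; ShadowBP is a floating shadow actor that appears when the player enters its trigger and speaks a dialog line.
; It fades out on BeginPlay, while a looping timeline bobs and rotates its core.
; Overlap by the main character runs ShowUp, which scales the core up, then enables Niagara effects and collision.
; Say then shows the keyed dialog on the player HUD and pops an instruction widget.
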(event `self.ReceiveBeginPlay`
  (bind _core (`self.Core`))
  (`|ExecutionSequence`
    (:`then_0`
      (bind (_direction _height) (`Timeline|InPlace` :!via `PlayFromStart` :!label _label)
        (:`Update`
          (`SceneComponent.K2_SetRelativeLocation` _core (`KismetMathLibrary.MakeVector` 0.0 0.0 _height) true false)
          (`SceneComponent.K2_AddRelativeRotation` _core (`KismetMathLibrary.MakeRotator` 1.0) false false))
        (:`Finished`
          (`|ExecutionSequence`
            (:`then_0`
              (goto _label :!via `PlayFromStart`))))))
    (:`then_1`
      (`self.FadeOut`))))

(event `Say`
  (params (Key :type String))
  (`/Game/Widgets/EB_PlayerHUD.ShowDialog` (`/Game/Characters/EBMainCharacter_BP.PlayerHUD` (cast `/Game/Characters/EBMainCharacter_BP` (`GameplayStatics.GetPlayerCharacter` 0) :!pure true)) Key)
  (`/Game/Widgets/InstructionWidget.Pop` (cast `/Game/Widgets/InstructionWidget` (`WidgetComponent.GetUserWidgetObject` (`self.Widget`)) :!pure true)))

(event `ShowUp`
  (bind _niagara (`self.Niagara`))
  (`self.SetActorHiddenInGame` false)
  (bind (_direction _size) (`Timeline|Expand` :!via `PlayFromStart`)
    (:`Update`
      (`SceneComponent.SetRelativeScale3D` (`self.Core`) _size))
    (:`Finished`
      (`SceneComponent.SetVisibility` _niagara true false)
      (`NiagaraComponent.SetPaused` _niagara false)
      (`PrimitiveComponent.SetCollisionEnabled` (`self.Sphere`) "QueryAndPhysics")
      (`self.Say` (`self.Key`)))))

(event `FadeOut`
  (bind _niagara (`self.Niagara`))
  (`SceneComponent.SetVisibility` _niagara false false)
  (`NiagaraComponent.SetPaused` _niagara true)
  (bind (_direction _size) (`Timeline|Fade` :!via `ReverseFromEnd`)
    (:`Update`
      (`SceneComponent.SetRelativeScale3D` (`self.Core`) _size))
    (:`Finished`
      (`PrimitiveComponent.SetCollisionEnabled` (`self.Sphere`) "NoCollision")
      (`self.SetActorHiddenInGame` true))))

(event `self.DialogTrigger.OnComponentBeginOverlap`
  (params (OverlappedComponent :type "PrimitiveComponent Object Reference") (OtherActor :type "Actor Object Reference") (OtherComp :type "PrimitiveComponent Object Reference") (OtherBodyIndex :type Integer) (bFromSweep :type Boolean) (SweepResult :type "HitResult Structure (by ref)"))
  (cast `/Game/Characters/EBMainCharacter_BP` OtherActor)
  (`self.ShowUp`))

(fn `UserConstructionScript`)